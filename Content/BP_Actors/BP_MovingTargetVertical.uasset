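; A shooting target actor that bobs up and down and awards the player when a projectile hits it.
; Tick moves it with a swept offset, flipping direction at bounds set 100 units above and below its spawn height.
; A hit from an actor tagged Projectile increments Score and Timer on the FirstPersonCharacter, then destroys the target.
; Otherwise it destroys itself five seconds after BeginPlay.
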(event `self.ReceiveBeginPlay`
  (bind _z (.z (`self.K2_GetActorLocation`)))
  (set `self.MinPositionZ` (- _z 100.0))
  (set `self.MaxPositionZ` (+ _z 100.0))
  (`KismetSystemLibrary.Delay` 5.0)
  (`self.K2_DestroyActor` :!label _label))

(event `self.ReceiveHit`
  (params (MyComp :type "PrimitiveComponent Object Reference") (Other :type "Actor Object Reference") (OtherComp :type "PrimitiveComponent Object Reference") (bSelfMoved :type Boolean) (HitLocation :type "Vector Structure") (HitNormal :type "Vector Structure") (NormalImpulse :type "Vector Structure") (Hit :type "HitResult Structure (by ref)"))
  (`KismetSystemLibrary.PrintString` "HIT")
  (if (`self.ActorHasTag` Other "Projectile")
    (bind _returnvalue (`GameplayStatics.GetActorOfClass` "/Game/FirstPersonBP/Blueprints/FirstPersonCharacter.FirstPersonCharacter_C"))
    (bind _output_get (set `/Game/FirstPersonBP/Blueprints/FirstPersonCharacter.Score` (+ (`/Game/FirstPersonBP/Blueprints/FirstPersonCharacter.Score` _returnvalue) 1) _returnvalue))
    (set `/Game/FirstPersonBP/Blueprints/FirstPersonCharacter.Timer` (+ (`/Game/FirstPersonBP/Blueprints/FirstPersonCharacter.Timer` _returnvalue) 1) _returnvalue)
    (goto _label)
    (else
      (`KismetSystemLibrary.PrintString` "not projectile"))))

(event `self.ReceiveTick`
  (params (DeltaSeconds :type "Float (single-precision)"))
  (bind _z (.z (`self.K2_GetActorLocation`)))
  (`self.K2_AddActorLocalOffset` (`KismetMathLibrary.MakeVector` 0.0 0.0 (* (`self.Direction`) 5.0)) true)
  (if (>= _z (`self.MaxPositionZ`))
    (set `self.Direction` -1.0)
    (`KismetSystemLibrary.PrintString` "Going down")
    (elif (<= _z (`self.MinPositionZ`))
      (set `self.Direction` 1.0)
      (`KismetSystemLibrary.PrintString` "Going up"))))

(fn `UserConstructionScript`)