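; BP_RedTarget is a short-lived shooting target that rewards the player with score and extra time.
; It destroys itself five seconds after BeginPlay unless hit earlier.
; A hit from an actor tagged Projectile looks up FirstPersonCharacter by class, increases its Score and Timer, then destroys the target.
; Debug prints report every hit and non-projectile contacts, and a disconnected TargetActor assignment never runs.
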(event `self.ReceiveBeginPlay`
  (`KismetSystemLibrary.Delay` 5.0)
  (`self.K2_DestroyActor` :!label _label))

(event `self.ReceiveHit`
  (params (MyComp :type "PrimitiveComponent Object Reference") (Other :type "Actor Object Reference") (OtherComp :type "PrimitiveComponent Object Reference") (bSelfMoved :type Boolean) (HitLocation :type "Vector Structure") (HitNormal :type "Vector Structure") (NormalImpulse :type "Vector Structure") (Hit :type "HitResult Structure (by ref)"))
  (`KismetSystemLibrary.PrintString` "HIT")
  (if (`self.ActorHasTag` Other "Projectile")
    (bind _returnvalue (`GameplayStatics.GetActorOfClass` "/Game/FirstPersonBP/Blueprints/FirstPersonCharacter.FirstPersonCharacter_C"))
    (bind _output_get (set `/Game/FirstPersonBP/Blueprints/FirstPersonCharacter.Score` (+ (`/Game/FirstPersonBP/Blueprints/FirstPersonCharacter.Score` _returnvalue) 1) _returnvalue))
    (set `/Game/FirstPersonBP/Blueprints/FirstPersonCharacter.Timer` (+ (`/Game/FirstPersonBP/Blueprints/FirstPersonCharacter.Timer` _returnvalue) 3) _returnvalue)
    (goto _label)
    (else
      (`KismetSystemLibrary.PrintString` "not projectile"))))

(fn `UserConstructionScript`)